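; Game mode for a gem-collecting level game, handling player stats, gem count, respawning and game over.
; BeginPlay counts emeralds, then uses the win volume's level index to capture pawn stats on the first level or restore lives and gems through BP_GameInstance on later ones.
; Respawn destroys the pawn and possesses a new one at the last checkpoint, falling back to the start point.
; Game over disables input and shows a widget with cursor.
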(event Custom|Respawn%20Player
  (Actor|DestroyActor (Game|Player|GetPlayerPawn 0))
  (CallFunction|ValidatedRespawnandPossess))

(event EventBeginPlay
  (CallFunction|GetRemainingGems)
  (bind _outactors (Actor|GetAllActorsOfClass "/Game/Blueprints/Actors/LevelTriggers/BP_WinVolume.BP_WinVolume_C"))
  (if (== (Default|GetCurrentLevelIndex (Utilities|Array|Get(acopy) _outactors (Variables|LevelRef|GetFirst%20Win%20Volume))) 0)
    (CallFunction|GetPlayerStats)
    (bind _asbp_game_instance (Utilities|Casting|CastToBP_GameInstance (Game|GetGameInstance)))
    (Default|GetStats _asbp_game_instance)
    (else
      (bind _asbp_game_instance_2 (Utilities|Casting|CastToBP_GameInstance (Game|GetGameInstance)))
      (Default|SetStats _asbp_game_instance_2)
      (CallFunction|SetPlayerStats)))
  (Development|PrintString "Make it to the end.  Don't leave any gems behind!!" true true "(R=1.000000,G=0.673491,B=0.000000,A=1.000000)" 4.0))

(event EventTick
  (params (DeltaSeconds :type Float%20%28single-precision%29)))

(fn ConstructionScript)

(fn GetPlayerStats
  (bind _asbp_player_pawn (Utilities|Casting|CastToBP_PlayerPawn (Game|Player|GetPlayerPawn 0)))
  (Variables|PlayerStats|SetPlayer%20HP (Variables|/Game/Blueprints/Actors/Pawns/BP_PlayerPawn.BP_PlayerPawn_C|GetHP _asbp_player_pawn))
  (Variables|PlayerStats|SetPlayer%20Max%20HP (Variables|/Game/Blueprints/Actors/Pawns/BP_PlayerPawn.BP_PlayerPawn_C|GetMaxHP _asbp_player_pawn))
  (Variables|PlayerStats|SetPlayer%20Lives (Variables|/Game/Blueprints/Actors/Pawns/BP_PlayerPawn.BP_PlayerPawn_C|GetLives _asbp_player_pawn))
  (Variables|PlayerStats|SetPlayer%20Location (Transformation|GetActorLocation _asbp_player_pawn))
  (Variables|PlayerStats|SetPlayer%20Gems%20Collected (Variables|/Game/Blueprints/Actors/Pawns/BP_PlayerPawn.BP_PlayerPawn_C|GetGems%20Collected _asbp_player_pawn)))

(fn SetPlayerStats
  (bind _asbp_player_pawn (Utilities|Casting|CastToBP_PlayerPawn (Game|Player|GetPlayerPawn 0)))
  (Variables|/Game/Blueprints/Actors/Pawns/BP_PlayerPawn.BP_PlayerPawn_C|SetLives _asbp_player_pawn (Variables|PlayerStats|GetPlayer%20Lives))
  (Variables|/Game/Blueprints/Actors/Pawns/BP_PlayerPawn.BP_PlayerPawn_C|SetGems%20Collected _asbp_player_pawn (Variables|PlayerStats|GetPlayer%20Gems%20Collected)))

(fn ValidatedRespawnandPossess
  (bind _last_checkpoint (Variables|LevelRef|GetLast%20Checkpoint)
    (:then
      (bind _returnvalue (Game|SpawnActorfromClass "/Game/Blueprints/Actors/Pawns/BP_PlayerPawn.BP_PlayerPawn_C" (Math|Transform|MakeTransform (.location (Transformation|GetWorldTransform (Variables|/Game/Blueprints/Actors/LevelTriggers/BP_Checkpoint.BP_Checkpoint_C|GetPOS _last_checkpoint))) (.rotation (Transformation|GetWorldTransform (Variables|/Game/Blueprints/Actors/LevelTriggers/BP_Checkpoint.BP_Checkpoint_C|GetPOS _last_checkpoint))) "1.000000,1.000000,1.000000") "AlwaysSpawn" "MultiplyWithRoot" 0 0))
      (Pawn|Possess (Game|GetPlayerController 0) _returnvalue))
    (:else
      (bind _start_point (Variables|LevelRef|GetStart%20Point)
        (:then
          (bind _returnvalue_2 (Game|SpawnActorfromClass "/Game/Blueprints/Actors/Pawns/BP_PlayerPawn.BP_PlayerPawn_C" (Math|Transform|MakeTransform (.location (Transformation|GetWorldTransform (Variables|/Game/Blueprints/Actors/LevelTriggers/BP_StartPoint.BP_StartPoint_C|GetPOS _start_point))) (.rotation (Transformation|GetWorldTransform (Variables|/Game/Blueprints/Actors/LevelTriggers/BP_StartPoint.BP_StartPoint_C|GetPOS _start_point))) "1.000000,1.000000,1.000000") "AlwaysSpawn" "MultiplyWithRoot" 0 0))
          (Pawn|Possess (Game|GetPlayerController 0) _returnvalue_2))
        (:else
          (bind _returnvalue_3 (Game|SpawnActorfromClass "/Game/Blueprints/Actors/Pawns/BP_PlayerPawn.BP_PlayerPawn_C" (Math|Transform|MakeTransform "0, 0, 0" "0, 0, 0" "1.000000,1.000000,1.000000") "AlwaysSpawn" "MultiplyWithRoot" 0 0))
          (Pawn|Possess (Game|GetPlayerController 0) _returnvalue_3))))))

(fn GameOver
  (bind _asbp_player_pawn (Utilities|Casting|CastToBP_PlayerPawn (Game|Player|GetPlayerPawn 0)))
  (Input|DisableInput _asbp_player_pawn (Game|GetPlayerController 0))
  (bind _returnvalue (UserInterface|CreateWidget "/Game/Blueprints/UI/WBP_GameOverScreen.WBP_GameOverScreen_C"))
  (UserInterface|Viewport|AddtoViewport _returnvalue 0)
  (Variables|/Script/Engine.PlayerController|SetbShowMouseCursor (Game|GetPlayerController 0) true))

(fn UpdateGemsUI
  (Variables|LevelRef|SetLevel%20Gems (- (Variables|LevelRef|GetLevel%20Gems) 1)))

(fn GetRemainingGems
  (bind _outactors (Actor|GetAllActorsOfClass "/Game/Blueprints/Actors/Collectables/BP_Emerald.BP_Emerald_C"))
  (Variables|LevelRef|SetLevel%20Gems (Utilities|Array|Length _outactors)))