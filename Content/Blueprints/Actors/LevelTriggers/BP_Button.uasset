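; BP_Button is a level trigger button that reveals FirstGap for a limited time when the player overlaps it.
; It refuses to press while Zone 1-tagged BP_Emerald actors remain, printing a warning instead.
; A timeline-driven Move Button graph lowers it, then delayed on-screen prints count down before FirstGap hides and the timeline reverses.
; A DoOnce, reset through IsButtonDown when the reverse finishes, blocks retriggering mid-cycle.
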(event OnComponentBeginOverlap(Button)
  (params (OverlappedComponent :type Primitive%20Component%20Object%20Reference) (OtherActor :type Actor%20Object%20Reference) (OtherComp :type Primitive%20Component%20Object%20Reference) (OtherBodyIndex :type Integer) (bFromSweep :type Boolean) (SweepResult :type Hit%20Result%20Structure%20%28by%20ref%29))
  (Utilities|IsPlayer OtherActor
    (:Player
      (bind _newparam (CallFunction|Zone1CrystalsRemaining))
      (if _newparam
        (Development|PrintString "Need to collect all Zone 1 Crystals first")
        (else
          (|MoveButton :!label _label
            (:else
              ;[1 0.02372 0.8404] Futre thoughts:  Convert this to UI
              (Variables|Default|SetIsButtonDown true)
              (Rendering|SetActorHiddenInGame (Variables|Default|GetFirstGap) false)
              (Development|PrintString "HURRY!!!" true true "(R=0.000000,G=0.364583,B=0.056446,A=1.000000)")
              (Utilities|FlowControl|Delay 12.0)
              (Development|PrintString "3..." true true "(R=0.000000,G=0.660000,B=1.000000,A=1.000000)" 1.0)
              (Utilities|FlowControl|Delay 1.0)
              (Development|PrintString "2..." true true "(R=0.000000,G=0.660000,B=1.000000,A=1.000000)" 1.0)
              (Utilities|FlowControl|Delay 1.0)
              (Development|PrintString "1..." true true "(R=0.000000,G=0.660000,B=1.000000,A=1.000000)" 1.0)
              (Utilities|FlowControl|Delay 1.0)
              (Rendering|SetActorHiddenInGame (Variables|Default|GetFirstGap) true)
              (goto _label Reverse))))))))

(fn ConstructionScript)

(fn Zone1CrystalsRemaining
  (bind _outactors (Actor|GetAllActorsOfClasswithTag "/Game/Blueprints/Actors/Collectables/BP_Emerald.BP_Emerald_C" "Zone 1"))
  (return (> (Utilities|Array|Length _outactors) 0)))