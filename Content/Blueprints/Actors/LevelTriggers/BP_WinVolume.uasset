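; BP_WinVolume is a level-exit trigger that responds when the player overlaps it.
; It checks for remaining BP_Emerald actors, printing a reminder if any exist and otherwise calling CompleteLevel.
; Helpers find the current level's index in a LevelNames array to detect the final level or open the next one.
; CompleteLevel only evaluates the final-level check so far, and LoadNextLevel is never called here.
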(event Collision|EventActorBeginOverlap
  (params (OtherActor :type Actor%20Object%20Reference))
  (Utilities|IsPlayer OtherActor
    (:Player
      (if (CallFunction|AnyEmeraldsRemaining)
        (Development|PrintString "Looks like there are still some gems to be collected")
        (else
          (CallFunction|CompleteLevel))))))

(fn ConstructionScript)

(fn AnyEmeraldsRemaining
  (bind _outactors (Actor|GetAllActorsOfClass "/Game/Blueprints/Actors/Collectables/BP_Emerald.BP_Emerald_C"))
  (return (> (Utilities|Array|Length _outactors) 0)))

(fn CompleteLevel
  (if (CallFunction|IsFinalLevel)
    _))

(fn GetCurrentLevelIndex
  (bind _returnvalue (Game|GetCurrentLevelName true))
  (return (Utilities|Array|FindItem (Variables|Default|GetLevel%20Names) (Utilities|String|StringToName _returnvalue))))

(fn IsFinalLevel
  (return (== (Utilities|Array|LastIndex (Variables|Default|GetLevel%20Names)) (CallFunction|GetCurrentLevelIndex))))

(fn LoadNextLevel
  (Game|OpenLevel(byName) (Utilities|Array|Get(acopy) (Variables|Default|GetLevel%20Names) (+ (CallFunction|GetCurrentLevelIndex) 1))))