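; BP_PlayerPawn is a physics-driven player pawn that rolls by torque and jumps by impulse.
; Tick rotates the spring arm camera from input and runs a short downward trace that gates jumping.
; Damage reduces HP or costs a life, syncing stats through BP_GameMode, which then respawns the player or ends the game.
; It also has helpers for spring arm adjustment and a fade-out level restart.
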(event EventBeginPlay
  (bind _asbp_game_mode (Utilities|Casting|CastToBP_GameMode (Game|GetGameMode)))
  (Variables|Default|SetBP%20GM%20Ref _asbp_game_mode)
  (CameraFades|StartCameraFade :self (Game|GetPlayerCameraManager 0) :FromAlpha 1.0 :Duration 3.0))

(event Game|Damage|EventAnyDamage
  (params (Damage :type Float%20%28single-precision%29) (DamageType :type Damage%20Type%20Object%20Reference) (InstigatedBy :type Controller%20Object%20Reference) (DamageCauser :type Actor%20Object%20Reference))
  ;[1 1 1] Damage system with any damage event.  Does health and lives check to respawn in level or restart
  (if (or (>= Damage (Variables|Default|GetHP)) (== (Variables|Default|GetHP) 0.0))
    (Variables|Default|SetLives (- (Variables|Default|GetLives) 1))
    (bind _as_bp_gamemode (CallFunction|UpdateStats))
    (if (> (Variables|/Game/Blueprints/Actors/GameModes/BP_GameMode.BP_GameMode_C|GetPlayer%20Lives _as_bp_gamemode) 0)
      (Default|RespawnPlayer _as_bp_gamemode)
      (else
        (Default|GameOver (Variables|Default|GetBP%20GM%20Ref))))
    (else
      (Variables|Default|SetHP (- (Variables|Default|GetHP) Damage))
      (CallFunction|UpdateStats))))

(event EventTick
  (params (DeltaSeconds :type Float%20%28single-precision%29))
  (bind _springarm (Variables|Default|GetSpringArm))
  (bind _returnvalue (Transformation|GetWorldLocation _springarm))
  (CallFunction|CameraMovement)
  (bind _returnvalue_2 (Collision|LineTraceByChannel _returnvalue (- _returnvalue "0.000000,0.000000,60.000000") "TraceTypeQuery1" false 0 "None"))
  (Variables|Default|SetIsOnGround _returnvalue_2))

(event Input|ActionEvents|InputActionJump
  (params (Key :type Key%20Structure :default "None"))
  (:Pressed
    (if (Variables|Default|GetIsOnGround)
      (Physics|AddImpulse (Variables|Default|GetPlayerAvatar) (Math|Vector|MakeVector 0.0 0.0 (Variables|Default|GetJump%20Force)) "None" true))))

(event Input|AxisEvents|InputAxisMoveForward/Backward
  (params (AxisValue :type Float%20%28single-precision%29))
  ;[0.1641 1 0.04246] Movement input times accel var to add torque
  (Class|PrimitiveComponent|AddTorqueinRadians (Variables|Default|GetPlayerAvatar) (Math|Vector|MakeVector 0.0 (* AxisValue (Variables|Default|GetAccel%20Mult)) 0.0) "None" true))

(event Input|AxisEvents|InputAxisMoveRight/Left
  (params (AxisValue :type Float%20%28single-precision%29))
  ;[0.1641 1 0.04246] Movement input times accel var to add torque
  (Class|PrimitiveComponent|AddTorqueinRadians (Variables|Default|GetPlayerAvatar) (Math|Vector|MakeVector (* AxisValue (Variables|Default|GetAccel%20Mult)) 0.0 0.0) "None" true))

(fn ConstructionScript)

(fn CameraMovement
  (bind _springarm (Variables|Default|GetSpringArm))
  (bind _returnvalue (Transformation|GetWorldRotation _springarm))
  (bind (_roll _pitch _yaw) (Math|Rotator|BreakRotator _returnvalue))
  (Transformation|SetWorldRotation (Variables|Default|GetSpringArm) (Math|Rotator|MakeRotator 0.0 (+ (Class|Actor|GetInputAxisKeyValue) _pitch) (+ _yaw (Class|Actor|GetInputAxisKeyValue))) false false))

(fn UpdateStats
  (bind _bp_gm_ref (Variables|Default|GetBP%20GM%20Ref))
  (Default|GetPlayerStats _bp_gm_ref)
  (Default|SetPlayerStats _bp_gm_ref)
  (return _bp_gm_ref))

(fn AdjustSpringArm
  (params (Distance :type Float%20%28double-precision%29) (Pitch :type Float%20%28double-precision%29))
  (bind _springarm (Variables|Default|GetSpringArm))
  (Variables|/Script/Engine.SpringArmComponent|SetTargetArmLength _springarm Distance)
  (Transformation|SetWorldRotation _springarm (Math|Rotator|MakeRotator 0.0 Pitch 0.0) false false))