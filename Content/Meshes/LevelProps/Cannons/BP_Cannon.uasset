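; BP_Cannon is a level prop cannon that automatically fires cannonballs on a repeating timer.
; After each FireRate delay, it spawns a BP_CannonBall at the spawn point with configurable scale and passes on its BaseDamage.
; The CannonAnim timeline then slides the barrel along its local Y axis, and its Cannon Fired event track restarts the delay, closing the firing loop.
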(event EventBeginPlay
  (Utilities|FlowControl|Delay (Variables|CannonProperties|GetFireRate) :!label _label)
  (CallFunction|SpawnCannonball)
  (bind _cannon (Timeline|CannonAnim PlayFromStart)
    (:Update
      (Transformation|SetRelativeLocation (Variables|Default|GetCannon_Barrel) (Math|Vector|MakeVector 0.0 _cannon 0.0) false false))
    (:CannonFired
      (goto _label))))

(fn ConstructionScript)

(fn SpawnCannonball
  (bind _projectilespawnpoint (Variables|Default|GetProjectileSpawnPoint))
  (bind _returnvalue (Game|SpawnActorfromClass "/Game/Blueprints/Actors/Projectiles/BP_CannonBall.BP_CannonBall_C" (Math|Transform|MakeTransform (Transformation|GetWorldLocation _projectilespawnpoint) (Transformation|GetWorldRotation _projectilespawnpoint) (Math|Conversions|ToVector(Float) (Variables|CannonProperties|GetProjectile%20Scale))) "Undefined" "MultiplyWithRoot" 0 0))
  (Variables|/Game/Blueprints/Actors/Projectiles/BP_CannonBall.BP_CannonBall_C|SetBase%20Damage _returnvalue (Variables|CannonProperties|GetBase%20Damage)))